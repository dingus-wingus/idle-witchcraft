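; Game instance that owns the save data for a potion-brewing game and exposes it through GetGameData.
; On Init it synchronously loads the BP_SaveGame slot, or creates a new save object if none exists.
; Per-field Save events cover progress such as tutorial, inventory, cauldron state, scenarios and coins, each writing to SavedData then saving immediately.
; Saves are synchronous, except tutorial, ingredient and potion saves, which can opt into async.
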(event `self.ReceiveInit`
  (`self.LoadGameData` false))

(event `/Game/_Blueprints/_Interfaces/BPI_SaveGame.LoadGameData`
  (params (Async :type Boolean))
  ;[0 0.000203 0.15 0.5] Load Game
  (bind _returnvalue (`GameplayStatics.DoesSaveGameExist` (`self.slotName`)))
  (if _returnvalue
    (if Async
      (bind _savegame (`AsyncActionHandleSaveGame.AsyncLoadGameFromSlot` (`self.slotName`))
        (:`Completed`
          (bind _asbp_save_game (cast `/Game/_Blueprints/Saving/BP_SaveGame` _savegame))
          (bind _output_get (set `self.savedData` _asbp_save_game))
          (set `/Game/_Blueprints/Saving/BP_SaveGame.saveGameExists` true _output_get)))
      (else
        (bind _returnvalue_2 (`GameplayStatics.LoadGameFromSlot` (`self.slotName`)))
        (bind _asbp_save_game_2 (cast `/Game/_Blueprints/Saving/BP_SaveGame` _returnvalue_2))
        (bind _output_get_2 (set `self.savedData` _asbp_save_game_2))
        (set `/Game/_Blueprints/Saving/BP_SaveGame.saveGameExists` true _output_get_2)))
    (else
      (bind _returnvalue_3 (`GameplayStatics.CreateSaveGameObject` "/Game/_Blueprints/Saving/BP_SaveGame.BP_SaveGame_C"))
      (set `self.savedData` _returnvalue_3))))

(event `/Game/_Blueprints/_Interfaces/BPI_SaveGame.SaveGameData`
  (params (Async :type Boolean))
  ;[0 0.005022 0.15 0.5] Save Game
  (if Async
    (`AsyncActionHandleSaveGame.AsyncSaveGameToSlot` (`self.savedData`) (`self.slotName`))
    (else
      (`GameplayStatics.SaveGameToSlot` (`self.savedData`) (`self.slotName`)))))

(event `/Game/_Blueprints/_Interfaces/BPI_SaveGame.SaveFirstLoad`
  (params (firstLoadComplete :type Boolean))
  (set `/Game/_Blueprints/Saving/BP_SaveGame.firstLoadSave` firstLoadComplete (`self.savedData`))
  (`/Game/_Blueprints/_Interfaces/BPI_SaveGame.SaveGameData` false))

(event `/Game/_Blueprints/_Interfaces/BPI_SaveGame.SaveTutorial`
  (params (tutorialSaveData :type "/Game/_Blueprints/_Structures/Struct_TutorialSave Structure") (Async :type Boolean))
  ;[0 0.002753 0.15 0.5] Get saved data from tutorial and update variable located here
  (set `/Game/_Blueprints/Saving/BP_SaveGame.tutorialSave` tutorialSaveData (`self.savedData`))
  (`/Game/_Blueprints/_Interfaces/BPI_SaveGame.SaveGameData` Async))

(event `/Game/_Blueprints/_Interfaces/BPI_SaveGame.SaveIngredients`
  (params (ingredientsArray :type "Array of /Game/_Blueprints/_Structures/Struct_ItemStats Structure (by ref)") (Async :type Boolean))
  ;[9e-06 0 0.15 0.5] Ingredients and potions saving
  (set `/Game/_Blueprints/Saving/BP_SaveGame.ingredientsSave` ingredientsArray (`self.savedData`))
  (`/Game/_Blueprints/_Interfaces/BPI_SaveGame.SaveGameData` Async))

(event `/Game/_Blueprints/_Interfaces/BPI_SaveGame.SavePotions`
  (params (potionsArray :type "Array of /Game/_Blueprints/_Structures/Struct_ItemStats Structure (by ref)") (Async :type Boolean))
  ;[9e-06 0 0.15 0.5] Ingredients and potions saving
  (set `/Game/_Blueprints/Saving/BP_SaveGame.potionsSave` potionsArray (`self.savedData`))
  (`/Game/_Blueprints/_Interfaces/BPI_SaveGame.SaveGameData` Async))

(event `/Game/_Blueprints/_Interfaces/BPI_SaveGame.SaveScene`
  (params (focusCamera :type "Actor Object Reference"))
  ;[0 0.01272 0.15 0.5] Save scene player is in
  (set `/Game/_Blueprints/Saving/BP_SaveGame.focusCameraSave` focusCamera (`self.savedData`))
  (`/Game/_Blueprints/_Interfaces/BPI_SaveGame.SaveGameData` false))

(event `/Game/_Blueprints/_Interfaces/BPI_SaveGame.SaveIconA`
  (params (icon :type "Texture2D Object Reference"))
  ;[0 0.002859 0.15 0.5] Save icons of items in cauldron
  (set `/Game/_Blueprints/Saving/BP_SaveGame.slotIconASave` icon (`self.savedData`))
  (`/Game/_Blueprints/_Interfaces/BPI_SaveGame.SaveGameData` false))

(event `/Game/_Blueprints/_Interfaces/BPI_SaveGame.SaveIconB`
  (params (icon :type "Texture2D Object Reference"))
  ;[0 0.002859 0.15 0.5] Save icons of items in cauldron
  (set `/Game/_Blueprints/Saving/BP_SaveGame.slotIconBSave` icon (`self.savedData`))
  (`/Game/_Blueprints/_Interfaces/BPI_SaveGame.SaveGameData` false))

(event `/Game/_Blueprints/_Interfaces/BPI_SaveGame.SaveCauldronIngredients`
  (params (cauldronIngredients :type "Array of /Game/_Blueprints/_Structures/Struct_ItemStats Structure (by ref)"))
  ;[0.003495 0 0.15 0.5] Save what ingredients are currently in cauldron
  (set `/Game/_Blueprints/Saving/BP_SaveGame.cauldronIngredientsSave` cauldronIngredients (`self.savedData`))
  (`/Game/_Blueprints/_Interfaces/BPI_SaveGame.SaveGameData` false))

(event `/Game/_Blueprints/_Interfaces/BPI_SaveGame.SaveDroppedSlots`
  (params (droppedSlots :type "Array of Integer (by ref)"))
  ;[0 0.006855 0.15 0.5] Save the slots that have been dropped into cauldron
  (set `/Game/_Blueprints/Saving/BP_SaveGame.droppedSlotsSave` droppedSlots (`self.savedData`))
  (`/Game/_Blueprints/_Interfaces/BPI_SaveGame.SaveGameData` false))

(event `/Game/_Blueprints/_Interfaces/BPI_SaveGame.SaveDiscoveredPotions`
  (params (discoveredPotions :type "Array of String (by ref)"))
  ;[0.01115 0.000412 0.15 0.5] Save discovered potions
  (set `/Game/_Blueprints/Saving/BP_SaveGame.discoveredPotionsSave` discoveredPotions (`self.savedData`))
  (`/Game/_Blueprints/_Interfaces/BPI_SaveGame.SaveGameData` false))

(event `/Game/_Blueprints/_Interfaces/BPI_SaveGame.SaveCurrentScenarioName`
  (params (currentSceneName :type Name))
  ;[0.009308 0 0.15 0.5] Scenario Saving
  (set `/Game/_Blueprints/Saving/BP_SaveGame.currentSceneNameSave` currentSceneName (`self.savedData`))
  (`/Game/_Blueprints/_Interfaces/BPI_SaveGame.SaveGameData` false))

(event `/Game/_Blueprints/_Interfaces/BPI_SaveGame.SaveSceneQueue`
  (params (SceneQueue :type "Array of Name (by ref)"))
  ;[0.009308 0 0.15 0.5] Scenario Saving
  (set `/Game/_Blueprints/Saving/BP_SaveGame.SceneQueueSave` SceneQueue (`self.savedData`))
  (`/Game/_Blueprints/_Interfaces/BPI_SaveGame.SaveGameData` false))

(event `/Game/_Blueprints/_Interfaces/BPI_SaveGame.SaveCoinAmount`
  (params (coinAmount :type Integer))
  ;[0.006425 0 0.15 0.5] Save coin amount
  (set `/Game/_Blueprints/Saving/BP_SaveGame.coinAmountSave` coinAmount (`self.savedData`))
  (`/Game/_Blueprints/_Interfaces/BPI_SaveGame.SaveGameData` false))

(fn `GetGameData`
  (returns (SaveGameData :type "/Game/_Blueprints/Saving/BP_SaveGame Object Reference"))
  (return (`self.savedData`)))