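; Core HUD that creates the main HUD, pause, inventory, potion, scenario, crafting and inventory-button widgets at BeginPlay.
; Menu and utility widgets are kept in separate lists, with open ones tracked in matching arrays.
; ToggleWidget shows one menu exclusively and collapses open utilities, while Open/Close events set visibility directly.
; PauseToggle hides tracked widgets and re-shows them on closing, and TogglePauseMenu sets game pause from the menu's visibility.
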(event `self.ReceiveBeginPlay`
  (`|ExecutionSequence`
    (:`then_0`
      ;[0 0.01949 0.15 0.5] Game
      (bind _returnvalue (`|CreateWidget` "/Game/_Blueprints/_Widgets/WB_Core_HUD.WB_Core_HUD_C" (`self.GetOwningPlayerController`)))
      (bind _output_get (set `self.wB_Core_HUD` _returnvalue))
      (`UserWidget.AddToViewport` _output_get 0))
    (:`then_1`
      ;[0 0.03517 0.15 0.5] Game Menu
      (bind _returnvalue_2 (`|CreateWidget` "/Game/_Blueprints/_Widgets/WB_PauseMenu.WB_PauseMenu_C" (`self.GetOwningPlayerController`)))
      (bind _output_get_2 (set `self.wB_PauseMenu` _returnvalue_2))
      (`KismetArrayLibrary.Array_Add` (`self.gameMenuWidgetList`) _output_get_2)
      (bind _returnvalue_3 (`|CreateWidget` "/Game/_Blueprints/_Inventory/WB_Inventory.WB_Inventory_C"))
      (bind _output_get_3 (set `self.wbInventory` _returnvalue_3))
      (`KismetArrayLibrary.Array_Add` (`self.gameMenuWidgetList`) _output_get_3)
      (bind _returnvalue_4 (`|CreateWidget` "/Game/_Blueprints/_Inventory/WB_PotionInventory.WB_PotionInventory_C"))
      (bind _output_get_4 (set `self.wBPotionInventory` _returnvalue_4))
      (`KismetArrayLibrary.Array_Add` (`self.gameMenuWidgetList`) _output_get_4)
      (bind _returnvalue_5 (`|CreateWidget` "/Game/_Data/_Scenarios/WB_Scenario.WB_Scenario_C"))
      (bind _output_get_5 (set `self.WB Scenario` _returnvalue_5))
      (`KismetArrayLibrary.Array_Add` (`self.gameMenuWidgetList`) _output_get_5)
      ;[0 0.005641 0.15 0.5] Add widgets to vieport (Defualted to hidden)
      (for _array_element (`self.gameMenuWidgetList`)
        (`UserWidget.AddToViewport` _array_element 0)))
    (:`then_2`
      ;[0 0.007725 0.15 0.5] Game Utilities
      (bind _returnvalue_6 (`|CreateWidget` :`Class` "/Game/_Blueprints/_Crafting/WB_CraftingManager.WB_CraftingManager_C" :`bPInventorymanager` null))
      (bind _output_get_6 (set `self.wBCraftingManager` _returnvalue_6))
      (`KismetArrayLibrary.Array_Add` (`self.gameUtilitiesWidgetList`) _output_get_6)
      (bind _returnvalue_7 (`|CreateWidget` "/Game/_Blueprints/_Inventory/WB_InventoryButtons.WB_InventoryButtons_C"))
      (bind _output_get_7 (set `self.wB_InventoryButtons` _returnvalue_7))
      (`KismetArrayLibrary.Array_Add` (`self.gameUtilitiesWidgetList`) _output_get_7)
      ;[0 0.005641 0.15 0.5] Add widgets to vieport (Defualted to hidden)
      (for _array_element_2 (`self.gameUtilitiesWidgetList`)
        (`UserWidget.AddToViewport` _array_element_2 0)))))

(event `TogglePauseMenu`
  (`self.PauseToggle` (`self.wB_PauseMenu`))
  (if (`Widget.IsVisible` (`self.wB_PauseMenu`))
    (`GameplayStatics.SetGamePaused` true)
    (else
      (`GameplayStatics.SetGamePaused` false))))

(event `CloseInventory`
  (bind _wbinventory (`self.wbInventory`))
  (`Widget.SetVisibility` _wbinventory "Collapsed")
  (`KismetArrayLibrary.Array_RemoveItem` (`self.OpennedMenuWidgets`) _wbinventory))

(event `ToggleInventory`
  (`self.ToggleWidget` (`self.wbInventory`)))

(event `OpenInventory`
  (bind _wbinventory (`self.wbInventory`))
  (`Widget.SetVisibility` _wbinventory "SelfHitTestInvisible")
  (`KismetArrayLibrary.Array_Add` (`self.OpennedMenuWidgets`) _wbinventory))

(event `TogglePotionsInventory`
  (`self.ToggleWidget` (`self.wBPotionInventory`)))

(event `OpenPotionsInventory`
  (bind _wbpotioninventory (`self.wBPotionInventory`))
  (`Widget.SetVisibility` _wbpotioninventory "SelfHitTestInvisible")
  (`KismetArrayLibrary.Array_Add` (`self.OpennedMenuWidgets`) _wbpotioninventory))

(event `ClosePotionsInventory`
  (bind _wbpotioninventory (`self.wBPotionInventory`))
  (`Widget.SetVisibility` _wbpotioninventory "Collapsed")
  (`KismetArrayLibrary.Array_RemoveItem` (`self.OpennedMenuWidgets`) _wbpotioninventory))

(event `CloseInventories`
  (`self.CloseInventory`)
  (`self.ClosePotionsInventory`)
  (`self.CloseInventoryButtons`))

(event `OpenInventoryButtons`
  (bind _wb_inventorybuttons (`self.wB_InventoryButtons`))
  (`Widget.SetVisibility` _wb_inventorybuttons "SelfHitTestInvisible")
  (`KismetArrayLibrary.Array_Add` (`self.OpennedUtilityWidgets`) _wb_inventorybuttons))

(event `CloseInventoryButtons`
  (bind _wb_inventorybuttons (`self.wB_InventoryButtons`))
  (`Widget.SetVisibility` _wb_inventorybuttons "Collapsed")
  (`KismetArrayLibrary.Array_RemoveItem` (`self.OpennedUtilityWidgets`) _wb_inventorybuttons))

(event `OpenCrafting`
  (bind _wbcraftingmanager (`self.wBCraftingManager`))
  (`Widget.SetVisibility` _wbcraftingmanager "SelfHitTestInvisible")
  (`KismetArrayLibrary.Array_Add` (`self.OpennedUtilityWidgets`) _wbcraftingmanager)
  (`Widget.SetVisibility` (`/Game/_Blueprints/_Crafting/WB_CraftingManager.backButton` _wbcraftingmanager) "SelfHitTestInvisible"))

(event `CloseCrafting`
  (bind _wbcraftingmanager (`self.wBCraftingManager`))
  (`Widget.SetVisibility` _wbcraftingmanager "Collapsed")
  (set `/Game/_Blueprints/_Crafting/WB_CraftingManager.crafting` false _wbcraftingmanager)
  (`KismetArrayLibrary.Array_RemoveItem` (`self.OpennedUtilityWidgets`) _wbcraftingmanager))

(event `ToggleScenario`
  (`self.ToggleWidget` (`self.WB Scenario`)))

(fn `FocusGame`
  (`Widget.SetVisibility` (`self.widgetToFocus`) "Collapsed"))

(fn `FocusWidget`
  (`Widget.SetVisibility` (`self.widgetToFocus`) "SelfHitTestInvisible"))

(fn `PauseToggle`
  (params (TargetWidget :type "UserWidget Object Reference"))
  (bind _opennedmenuwidgets (`self.OpennedMenuWidgets`))
  (`/Engine/EditorBlueprintResources/StandardMacros.IsValid` TargetWidget
    (:`Is Valid`
      (set `self.widgetToFocus` TargetWidget)
      (for _array_element (`self.gameMenuWidgetList`)
        (`/Engine/EditorBlueprintResources/StandardMacros.IsValid` _array_element
          (:`Is Valid`
            (if (== (`self.widgetToFocus`) _array_element)
              (if (`Widget.IsVisible` (`self.widgetToFocus`))
                (`self.FocusGame`)
                ;[0.000243 0 0.15 0.5] Hide and show old widgets if pause is open
                (for _array_element_2 _opennedmenuwidgets
                  (`Widget.SetVisibility` _array_element_2 "SelfHitTestInvisible")
                  (`KismetArrayLibrary.Array_Clear` _opennedmenuwidgets)
                  (for _array_element_3 (`self.OpennedUtilityWidgets`)
                    (`Widget.SetVisibility` _array_element_3 "SelfHitTestInvisible")))
                (else
                  (`self.FocusWidget`)
                  (for _array_element_4 (`self.OpennedMenuWidgets`)
                    (`Widget.SetVisibility` _array_element_4 "Collapsed")
                    (for _array_element_5 (`self.OpennedUtilityWidgets`)
                      (`Widget.SetVisibility` _array_element_5 "Collapsed")))))
              (elif (`Widget.IsVisible` _array_element)
                (`KismetArrayLibrary.Array_Add` (`self.OpennedMenuWidgets`) _array_element)
                (`KismetArrayLibrary.Array_Add` (`self.OpennedUtilityWidgets`) _array_element)))))))))

(fn `ToggleWidget`
  (params (TargetWidget :type "UserWidget Object Reference"))
  (bind _opennedmenuwidgets (`self.OpennedMenuWidgets`))
  (bind _opennedutilitywidgets (`self.OpennedUtilityWidgets`))
  (`/Engine/EditorBlueprintResources/StandardMacros.IsValid` TargetWidget
    (:`Is Valid`
      (set `self.widgetToFocus` TargetWidget)
      (for _array_element (`self.gameMenuWidgetList`)
        (`/Engine/EditorBlueprintResources/StandardMacros.IsValid` _array_element
          (:`Is Valid`
            (if (== (`self.widgetToFocus`) _array_element)
              (if (`Widget.IsVisible` (`self.widgetToFocus`))
                (`self.FocusGame`)
                ;[0 0.01212 0.15 0.5] Store whether a widget is open or not in array
                (`KismetArrayLibrary.Array_RemoveItem` (`self.OpennedMenuWidgets`) (`self.widgetToFocus`))
                (else
                  (`self.FocusWidget`)
                  (`KismetArrayLibrary.Array_Clear` _opennedmenuwidgets)
                  (`KismetArrayLibrary.Array_Add` _opennedmenuwidgets (`self.widgetToFocus`))
                  (for _array_element_2 _opennedutilitywidgets
                    (`Widget.SetVisibility` _array_element_2 "Collapsed")
                    (`KismetArrayLibrary.Array_RemoveItem` _opennedutilitywidgets _array_element_2))))
              (elif (`Widget.IsVisible` _array_element)
                (`Widget.SetVisibility` _array_element "Collapsed")))))))))

(fn `UserConstructionScript`)