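; Player Blueprint whose only active logic is a pause menu toggle on the IA_Pause Enhanced Input action.
; The IsPauseMenuOpen flag alternates between creating a new WB_PauseMenu with the game paused and removing it to resume.
; Input mode switches between Game and UI and Game Only, while the mouse cursor is set visible on both opening and closing.
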(event `EnhancedInput|/Game/_Blueprints/_InputActions/IA_Pause`
  (params (ActionValue :type Boolean) (ElapsedSeconds :type "Float (double-precision)") (TriggeredSeconds :type "Float (double-precision)") (InputAction :type "InputAction Object Reference" :default "/Game/_Blueprints/_InputActions/IA_Pause.IA_Pause"))
  (bind _returnvalue (`GameplayStatics.GetPlayerController` 0))
  ;[0.15 0.1367 0.01598 0.5] Pause Menu
  (:`Started`
    (if (not (`self.isPauseMenuOpen`))
      (set `self.isPauseMenuOpen` true)
      (bind _returnvalue_2 (`|CreateWidget` "/Game/_Blueprints/WB_PauseMenu.WB_PauseMenu_C" _returnvalue))
      (bind _output_get (set `self.pauseMenuWidget` _returnvalue_2))
      (`UserWidget.AddToViewport` _output_get 0)
      (`WidgetBlueprintLibrary.SetInputMode_GameAndUIEx` _returnvalue (`self.pauseMenuWidget`))
      (set `PlayerController.bShowMouseCursor` true (`GameplayStatics.GetPlayerController` 0))
      (`GameplayStatics.SetGamePaused` true)
      (else
        (set `self.isPauseMenuOpen` false)
        (`Widget.RemoveFromParent` (`self.pauseMenuWidget`))
        (`GameplayStatics.SetGamePaused` false)
        (`WidgetBlueprintLibrary.SetInputMode_GameOnly` _returnvalue)
        (set `PlayerController.bShowMouseCursor` true (`GameplayStatics.GetPlayerController` 0))))))

(fn `UserConstructionScript`)