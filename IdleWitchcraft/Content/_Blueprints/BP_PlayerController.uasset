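; Player controller that lets the player tap or left-click world objects to interact with them.
; On BeginPlay it adds the IMC_Controls mapping context and caches the HUD core, but clicks use raw key events, noted as an Enhanced Input workaround.
; A cursor visibility trace finds the actor and messages it through BPI_Interact.
; RefreshInputs runs a self-restarting delay loop that flushes player input while not interacting.
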(event `self.ReceiveBeginPlay`
  (`self.InputSetup`)
  (bind _asbp_hud_core (`/Game/_Blueprints/_MacroLibrary/BML_GetHUDCorePLAYERCONTROLLER.Get_BP_HUD_Core` 10.0)
    (:`Success`
      (set `self.bP HUD Core` _asbp_hud_core))))

(event `Key|Touch1`
  (params (Key :type "Key Structure"))
  ;[0.004672 0 0.15 0.5] Enhanced System not working
  (:`Pressed`
    (`KismetSystemLibrary.PrintString` "Hello" :!label _label)
    ;[0 0.01695 0.75 0.5] Check if there is an object and if it is interactable then call interact
    (bind (_isfound _clikedactor) (`self.GetClickedActor`))
    (bind _output_get (set `self.Cliked Actor` _clikedactor))
    (if _isfound
      (bind _output_get_2 (set `self.canInteract` (`KismetSystemLibrary.DoesImplementInterface` _output_get "/Game/_Blueprints/_Interfaces/BPI_Interact.BPI_Interact_C")))
      (if _output_get_2
        (message `/Game/_Blueprints/_Interfaces/BPI_Interact.inInteract` (`self.Cliked Actor`))))))

(event `EnhancedInput|/Game/_Blueprints/_InputActions/IA_Interact`
  (params (ActionValue :type Boolean) (ElapsedSeconds :type "Float (double-precision)") (TriggeredSeconds :type "Float (double-precision)") (InputAction :type "InputAction Object Reference" :default "/Game/_Blueprints/_InputActions/IA_Interact.IA_Interact"))
  ;[0.004672 0 0.15 0.5] Enhanced System not working
)

(event `Key|LeftMouseButton`
  (params (Key :type "Key Structure"))
  ;[0.004672 0 0.15 0.5] Enhanced System not working
  (:`Pressed`
    (goto _label)))

(event `RefreshInputs`
  (`KismetSystemLibrary.Delay` 0.1 :!label _label_2)
  (`/Game/_Blueprints/_MacroLibrary/BML_DelayLoopACTOR.DelayLoop` 0.1 (not (`self.interacting`))
    (:`Loop Body`
      (`EnhancedInputLibrary.FlushPlayerInput` self))
    (:`False`
      (goto _label_2))))

(fn `GetClickedActor`
  (returns (isFound :type Boolean) (ClikedActor :type "Actor Object Reference"))
  (bind (_bblockinghit _binitialoverlap _time _distance _location _impactpoint _normal _impactnormal _physmat _hitactor) (`GameplayStatics.BreakHitResult` (`self.GetHitResultUnderCursorByChannel` "TraceTypeQuery1")))
  (return _bblockinghit _hitactor))

(fn `InputSetup`
  (bind _returnvalue (subsystem `EnhancedInputLocalPlayerSubsystem`))
  (`/Engine/EditorBlueprintResources/StandardMacros.IsValid` _returnvalue
    (:`Is Valid`
      (`EnhancedInputSubsystemInterface.AddMappingContext` _returnvalue "/Game/_Blueprints/_InputActions/IMC_Controls.IMC_Controls" 0 (struct)))))

(fn `UserConstructionScript`)