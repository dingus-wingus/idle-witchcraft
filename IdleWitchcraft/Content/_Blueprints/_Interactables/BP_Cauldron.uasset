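; BP_Cauldron is an interactable cauldron that opens the crafting mode.
; Interaction is ignored while the tutorial widget or a tooltip is open, and starts the crafting tutorial if it is not yet complete.
; It blends the view to BP_CraftingCam, saves that camera through the game instance, then flags the crafting manager and rearranges the HUD to show inventory and crafting together.
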(event `self.ReceiveBeginPlay`
  (bind _asbp_player_controller (`/Game/_Blueprints/_MacroLibrary/BML_GetPlayerControllerACTOR.GetBPPlayerController` 10.0)
    (:`Success`
      (set `self.bP Player Controller` _asbp_player_controller)
      (bind _returnvalue (`GameplayStatics.GetActorOfClass` "/Game/_Blueprints/Tutorial/BP_TutorialManager.BP_TutorialManager_C"))
      (set `self.bPTutorialManger` _returnvalue))))

(event `/Game/_Blueprints/_Interfaces/BPI_Interact.inInteract`
  (`self.OnInteract`))

(fn `OnInteract`
  (bind _bp_hud_core (`/Game/_Blueprints/BP_PlayerController.bP HUD Core` (`self.bP Player Controller`)))
  (bind _wbcraftingmanager (`/Game/_Blueprints/BP_HUD_Core.wBCraftingManager` (`/Game/_Blueprints/BP_PlayerController.bP HUD Core` (`self.bP Player Controller`))))
  (bind _wbcraftingmanager_2 (`/Game/_Blueprints/BP_HUD_Core.wBCraftingManager` _bp_hud_core))
  (if (and (not (`Widget.IsVisible` (`/Game/_Blueprints/Tutorial/BP_TutorialManager.wbTutorial` (`self.bPTutorialManger`)))) (not (`/Game/_Blueprints/BP_HUD_Core.toolTipOpen` (`/Game/_Blueprints/BP_PlayerController.bP HUD Core` (`self.bP Player Controller`)))))
    ;[0 0.004733 0.4253] Check if tutorial has happened
    (if (not (`/Game/_Blueprints/Tutorial/BP_TutorialManager.craftingTutorialComplete` (`self.bPTutorialManger`)))
      (`/Game/_Blueprints/Tutorial/BP_TutorialManager.PlayCraftingTutorial` (`self.bPTutorialManger`) 0))
    (set `/Game/_Blueprints/_Crafting/WB_CraftingManager.crafting` true _wbcraftingmanager)
    (set `/Game/_Blueprints/_Crafting/WB_CraftingManager.inMainScene` false _wbcraftingmanager)
    (`self.SwitchToCraftCam`)
    (`Widget.SetRenderTranslation` (`/Game/_Blueprints/_Inventory/WB_Inventory.inventoryWrapBox` (`/Game/_Blueprints/BP_HUD_Core.wbInventory` _bp_hud_core)) (50.0 200.0))
    ;[0 0.00596 0.15 0.5] close other widget but make sure inv is open
    (`/Game/_Blueprints/BP_HUD_Core.CloseInventories` _bp_hud_core)
    (`/Game/_Blueprints/BP_HUD_Core.ToggleInventory` _bp_hud_core)
    (`/Game/_Blueprints/BP_HUD_Core.OpenCrafting` _bp_hud_core)
    (`Widget.SetVisibility` (`/Game/_Blueprints/_Crafting/WB_CraftingManager.DropImage` _wbcraftingmanager_2) "Visible")
    ;[0 0.0101 0.15 0.5] Move progress bar back to center
    (`Widget.SetRenderTranslation` (`/Game/_Blueprints/_Crafting/WB_CraftingManager.ProgressBar` _wbcraftingmanager_2) (0.0 0.0))))

(fn `SwitchToCraftCam`
  ;[0 0.002387 0.15 0.5] Switch cam
  (bind _returnvalue (`GameplayStatics.GetActorOfClass` "/Game/_Blueprints/Cameras/BP_CraftingCam.BP_CraftingCam_C"))
  (bind _output_get (set `self.craftCam` _returnvalue))
  (`PlayerController.SetViewTargetWithBlend` (`GameplayStatics.GetPlayerController` 0) _output_get 0.0 "VTBlend_Linear" 0.0 false)
  (message `/Game/_Blueprints/_Interfaces/BPI_SaveGame.SaveScene` (`GameplayStatics.GetGameInstance`) (`self.craftCam`)))

(fn `UserConstructionScript`)