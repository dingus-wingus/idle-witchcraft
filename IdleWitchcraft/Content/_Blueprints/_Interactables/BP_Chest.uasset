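; BP_Chest is an interactable chest that toggles the player's inventory UI.
; On BeginPlay it caches the player controller and finds the tutorial manager in the level.
; Its interact event is ignored while the tutorial widget is visible; otherwise it toggles the inventory through the controller's HUD core.
; It then opens or closes the inventory buttons to match the inventory widget's visibility.
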(event `self.ReceiveBeginPlay`
  (bind _asbp_player_controller (`/Game/_Blueprints/_MacroLibrary/BML_GetPlayerControllerACTOR.GetBPPlayerController` 10.0)
    (:`Success`
      (set `self.bP Player Controller` _asbp_player_controller)
      (bind _returnvalue (`GameplayStatics.GetActorOfClass` "/Game/_Blueprints/Tutorial/BP_TutorialManager.BP_TutorialManager_C"))
      (set `self.tutorialManager` _returnvalue))))

(event `/Game/_Blueprints/_Interfaces/BPI_Interact.inInteract`
  (bind _bp_hud_core (`/Game/_Blueprints/BP_PlayerController.bP HUD Core` (`self.bP Player Controller`)))
  (bind _bp_hud_core_2 (`/Game/_Blueprints/BP_PlayerController.bP HUD Core` (`self.bP Player Controller`)))
  (if (not (`Widget.IsVisible` (`/Game/_Blueprints/Tutorial/BP_TutorialManager.wbTutorial` (`self.tutorialManager`))))
    (`KismetSystemLibrary.PrintString` "chest")
    (`/Game/_Blueprints/BP_HUD_Core.ToggleInventory` _bp_hud_core_2)
    ;[0 0.007304 0.15 0.5] If inventory is closing or openning then do the same with the buttons
    (if (`Widget.IsVisible` (`/Game/_Blueprints/BP_HUD_Core.wbInventory` _bp_hud_core_2))
      (`/Game/_Blueprints/BP_HUD_Core.OpenInventoryButtons` _bp_hud_core)
      (else
        (`/Game/_Blueprints/BP_HUD_Core.CloseInventoryButtons` _bp_hud_core)))))

(fn `UserConstructionScript`)