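; Interactable door that switches the player into the scenario view.
; On BeginPlay it caches the scenario handler and scenario camera actors found in the level.
; A valid interaction plays a door cue if sound is on, blends the view to the scenario camera and saves it via the GameInstance.
; It also reparents the potion inventory's wrap box from the middle to the high scale box and toggles the scenario HUD.
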(event `self.ReceiveBeginPlay`
  (`parent.ReceiveBeginPlay`)
  (bind _returnvalue (`GameplayStatics.GetActorOfClass` "/Game/_Data/_Scenarios/BP_ScenarioHandler.BP_ScenarioHandler_C"))
  (set `self.scenarioHandler` _returnvalue)
  (bind _returnvalue_2 (`GameplayStatics.GetActorOfClass` "/Game/_Blueprints/Cameras/BP_ScenarioCamera.BP_ScenarioCamera_C"))
  (set `self.scenarioCam` _returnvalue_2))

(event `/Game/_Blueprints/_Interfaces/BPI_Interact.inInteract`
  (`self.OnInteract`))

(fn `OnInteract`
  (bind _wbpotioninventory (`/Game/_Blueprints/BP_HUD_Core.wBPotionInventory` (`/Game/_Blueprints/BP_PlayerController.bP HUD Core` (`self.player Controller`))))
  (bind _potionswrapbox (`/Game/_Blueprints/_Inventory/WB_PotionInventory.potionsWrapBox` _wbpotioninventory))
  (bind _interactable (`self.CheckForInteraction`))
  (if _interactable
    (bind _asbp_game_instance_core (cast `/Game/_Blueprints/BP_GameInstanceCore` (`GameplayStatics.GetGameInstance`)))
    (if (`/Game/_Blueprints/BP_GameInstanceCore.soundOn` _asbp_game_instance_core)
      (`GameplayStatics.PlaySound2D` "/Game/_Sounds/SFX/Cue_Door.Cue_Door" 1.0 1.0 0.0 null null))
    (`PlayerController.SetViewTargetWithBlend` (`GameplayStatics.GetPlayerController` 0) (`self.scenarioCam`) 0.0 "VTBlend_Linear" 0.0 false)
    (message `/Game/_Blueprints/_Interfaces/BPI_SaveGame.SaveScene` (`GameplayStatics.GetGameInstance`) (`self.scenarioCam`))
    ;[0 0.01532 0.15 0.5] Add inventory to high scale box so we can move inventory across all sizes
    (`PanelWidget.AddChild` (`/Game/_Blueprints/_Inventory/WB_PotionInventory.highInventory` _wbpotioninventory) _potionswrapbox)
    (`PanelWidget.RemoveChild` (`/Game/_Blueprints/_Inventory/WB_PotionInventory.middleInventory` _wbpotioninventory) _potionswrapbox)
    (`/Game/_Blueprints/BP_HUD_Core.ToggleScenario` (`/Game/_Blueprints/BP_PlayerController.bP HUD Core` (`self.player Controller`)))))

(fn `UserConstructionScript`)