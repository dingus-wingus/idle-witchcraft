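; BP_Interactable is an interactable Blueprint, apparently a base, that gates interaction against open UI.
; On BeginPlay it caches the player controller and, once that succeeds, the tutorial manager.
; CheckForInteraction returns true only when neither a HUD tooltip nor the shop is open.
; When interaction is allowed, the check also clears any valid tutorial tapping indicator through the tutorial manager.
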(event `self.ReceiveBeginPlay`
  (bind _asbp_player_controller (`/Game/_Blueprints/_MacroLibrary/BML_GetPlayerControllerACTOR.GetBPPlayerController` 10.0)
    (:`Success`
      (set `self.player Controller` _asbp_player_controller)
      (bind _returnvalue (`GameplayStatics.GetActorOfClass` "/Game/_Blueprints/Tutorial/BP_TutorialManager.BP_TutorialManager_C"))
      (set `self.tutorialManager` _returnvalue))))

(fn `CheckForInteraction`
  (returns (Interactable :type Boolean))
  (bind _returnvalue (and (not (`/Game/_Blueprints/BP_HUD_Core.toolTipOpen` (`/Game/_Blueprints/BP_PlayerController.bP HUD Core` (`self.player Controller`)))) (not (`Widget.IsVisible` (`/Game/_Blueprints/BP_HUD_Core.wB_Shop` (`/Game/_Blueprints/BP_PlayerController.bP HUD Core` (`self.player Controller`)))))))
  (if _returnvalue
    (`self.RemoveVisualIndicator`))
  (return _returnvalue))

(fn `RemoveVisualIndicator`
  (if (`KismetSystemLibrary.IsValid` (`/Game/_Blueprints/Tutorial/BP_TutorialManager.wbTappingIndicator` (`self.tutorialManager`)))
    (`/Game/_Blueprints/Tutorial/BP_TutorialManager.RemoveTapping` (`self.tutorialManager`))))

(fn `UserConstructionScript`)