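; BP_Map is an interactable map actor that responds to the interact event.
; On BeginPlay it caches the player controller through a lookup taking a 10-second argument, then finds the tutorial manager in the level.
; Interaction is blocked while the tutorial widget is visible; otherwise it only prints a debug message that the map opened.
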(event `self.ReceiveBeginPlay`
  (bind _asbp_player_controller (`/Game/_Blueprints/_MacroLibrary/BML_GetPlayerControllerACTOR.GetBPPlayerController` 10.0)
    (:`Success`
      (set `self.bP Player Controller` _asbp_player_controller)
      (bind _returnvalue (`GameplayStatics.GetActorOfClass` "/Game/_Blueprints/Tutorial/BP_TutorialManager.BP_TutorialManager_C"))
      (set `self.tutorialManager` _returnvalue))))

(event `/Game/_Blueprints/_Interfaces/BPI_Interact.inInteract`
  (if (not (`Widget.IsVisible` (`/Game/_Blueprints/Tutorial/BP_TutorialManager.wbTutorial` (`self.tutorialManager`))))
    (`KismetSystemLibrary.PrintString` "Map Openned")))

(fn `UserConstructionScript`)