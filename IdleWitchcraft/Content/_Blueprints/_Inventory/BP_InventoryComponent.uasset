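; Inventory component that holds an eight-slot Items array of ingredient structs and displays it in a WB_Inventory widget created on BeginPlay.
; AddGinger and AddOlive run at startup, copying stats from placed BP_Ginger and BP_Olive actors into the first and last slots.
; Each add reloads the widget from the component.
; AddItem is an empty stub, and a ginger stacking loop capped at 99 is disconnected and never runs.
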(event `self.ReceiveBeginPlay`
  (bind _returnvalue (`|CreateWidget` "/Game/_Blueprints/_Inventory/_Widgets/WB_Inventory.WB_Inventory_C" null null))
  (bind _output_get (set `self.inventoryWidgetRef` _returnvalue))
  (`UserWidget.AddToViewport` _output_get 0)
  (`KismetArrayLibrary.Array_Resize` (`self.items`) 8)
  (`/Game/_Blueprints/_Inventory/_Widgets/WB_Inventory.LoadInventory` (`self.inventoryWidgetRef`) self)
  (`self.AddGinger`)
  (`self.AddOlive`))

(event `AddGinger`
  ;[0.15 0.08844 0.000631 0.5] Event to add specific ingredient
  (bind _returnvalue (`GameplayStatics.GetActorOfClass` "/Game/_Blueprints/_Inventory/Items/BP_Ginger.BP_Ginger_C"))
  (bind (_name _icon _amount _discovered _rarity _slotempty) (break `/Game/_Blueprints/_Inventory/Items/Struct_Item` (`/Game/_Blueprints/_Inventory/Items/BP_Ginger.gingerStats` _returnvalue)))
  (`KismetArrayLibrary.Array_Set` (`self.items`) 0 (make `/Game/_Blueprints/_Inventory/Items/Struct_Item` _name _icon _amount _discovered _rarity _slotempty))
  (`/Game/_Blueprints/_Inventory/_Widgets/WB_Inventory.LoadInventory` (`self.inventoryWidgetRef`) self))

(event `AddItem`)

(event `AddOlive`
  (bind _returnvalue (`GameplayStatics.GetActorOfClass` "/Game/_Blueprints/_Inventory/Items/BP_Olive.BP_Olive_C"))
  (bind (_name _icon _amount _discovered _rarity _slotempty) (break `/Game/_Blueprints/_Inventory/Items/Struct_Item` (`/Game/_Blueprints/_Inventory/Items/BP_Olive.oliveStats` _returnvalue)))
  (`KismetArrayLibrary.Array_Set` (`self.items`) 7 (make `/Game/_Blueprints/_Inventory/Items/Struct_Item` _name _icon _amount _discovered _rarity _slotempty))
  (`/Game/_Blueprints/_Inventory/_Widgets/WB_Inventory.LoadInventory` (`self.inventoryWidgetRef`) self))