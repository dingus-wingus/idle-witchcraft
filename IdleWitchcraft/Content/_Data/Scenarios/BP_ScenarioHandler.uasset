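; Debug simulation of branching customer dialogue scenarios, shown entirely through on-screen print strings.
; Pops row names from a scene queue, and ENTER starts or resolves each scenario using its DT_Test data table row.
; W and L toggle success or failure, which picks the outcome dialogue and the comma-separated follow-up scenarios appended to the queue.
; Older inline copies of the begin and resolve logic remain unconnected in the event graph.
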(event `self.ReceiveBeginPlay`
  (`KismetSystemLibrary.PrintString` "Starting Scenario Simulation...")
  (`KismetSystemLibrary.Delay` (`self.DelayBetween`))
  (`self.PopNextScenario`))

(event `Key|Enter`
  (params (Key :type "Key Structure"))
  ; Handle ENTER Input
  (:`Pressed`
    (switch `/Game/_Data/Scenarios/E_ScenarioState` (`self.State`)
      (:`NewEnumerator1`
        (`self.BeginScenario`))
      (:`NewEnumerator3`
        (`self.ResolveScenario`)
        (`KismetSystemLibrary.Delay` (`self.DelayBetween`))
        (`self.PopNextScenario`)))))

(event `Key|W`
  (params (Key :type "Key Structure"))
  ;[0.15 0.15 0.15 0.5 33] Change Win/Loss State
  (:`Pressed`
    (if (`|EnumEquality` (`self.State`) "NewEnumerator3")
      (set `self.ScenarioSucceeded` true)
      (`KismetSystemLibrary.PrintString` "(Scenario will Succeed. Press ENTER to Continue, or L to change)" true true (struct :`R` 1.0 :`G` 0.814847 :`A` 1.0)))))

(event `Key|L`
  (params (Key :type "Key Structure"))
  ;[0.15 0.15 0.15 0.5 33] Change Win/Loss State
  (:`Pressed`
    (if (`|EnumEquality` (`self.State`) "NewEnumerator3")
      (set `self.ScenarioSucceeded` false)
      (`KismetSystemLibrary.PrintString` "(Scenario will Fail. Press ENTER to Continue, or W to change)" true true (struct :`R` 1.0 :`G` 0.814847 :`A` 1.0)))))

(fn `BeginScenario`
  (bind _scenario_data (`self.GetCurrentScenario`))
  (bind (_scenarioname _dialogue _pointsrequired _statmultiplier _successdialogue _failuredialogue _charactersprite _unlockedscenariosonsuccess _unlockedscenariosonfailure _charactername) (break `/Game/_Data/Scenarios/F_Scenarios` _scenario_data))
  (`KismetSystemLibrary.PrintString` (`KismetStringLibrary.Concat_StrStr` _charactername ": " _dialogue) true true (struct :`G` 0.66 :`B` 1.0 :`A` 1.0) 5.0)
  (set `self.State` "NewEnumerator3")
  (if (`self.ScenarioSucceeded`)
    (`KismetSystemLibrary.PrintString` "(Scenario will Succeed. Press Enter to Continue, or L to change)" true true (struct :`R` 1.0 :`G` 0.814847 :`A` 1.0))
    (else
      (`KismetSystemLibrary.PrintString` "(Scenario will Fail. Press Enter to Continue, or W to change)" true true (struct :`R` 1.0 :`G` 0.814847 :`A` 1.0)))))

(fn `GetCurrentScenario`
  (returns (`Scenario Data` :type "/Game/_Data/Scenarios/F_Scenarios Structure"))
  (bind _currentscenename (`self.CurrentSceneName`))
  (bind _returnvalue (`|GetDataTableRow` "/Game/_Data/Scenarios/DT_Test.DT_Test" _currentscenename)
    (:`then`
      (return _returnvalue))
    (:`RowNotFound`
      (`KismetSystemLibrary.PrintString` (`KismetStringLibrary.Concat_StrStr` "Data Table contains no row named: " (`KismetStringLibrary.Conv_NameToString` _currentscenename)) true true (struct :`R` 1.0 :`G` 0.022658 :`A` 1.0)))))

(fn `PopNextScenario`
  (bind _scenequeue (`self.SceneQueue`))
  (if (`KismetArrayLibrary.Array_IsNotEmpty` _scenequeue)
    (set `self.CurrentSceneName` (`|GetArrayItem` _scenequeue))
    (`KismetArrayLibrary.Array_Remove` (`self.SceneQueue`))
    (`KismetSystemLibrary.PrintString` "A customer is here! Press ENTER to speak with them" true true (struct :`G` 1.0 :`B` 0.071252 :`A` 1.0))
    (set `self.State` "NewEnumerator1")
    (else
      (`KismetSystemLibrary.PrintString` "Scene Queue Empty! Stopping Senario Simulation"))))

(fn `ResolveScenario`
  (bind _scenario_data (`self.GetCurrentScenario`))
  (if (`self.ScenarioSucceeded`)
    (bind (_scenarioname _dialogue _pointsrequired _statmultiplier _successdialogue _failuredialogue _charactersprite _unlockedscenariosonsuccess _unlockedscenariosonfailure) (break `/Game/_Data/Scenarios/F_Scenarios` _scenario_data))
    (`KismetSystemLibrary.PrintString` _successdialogue true true (struct :`G` 1.0 :`B` 0.042616 :`A` 1.0))
    ; Add Unlocked Scenarios to Scene Queue (Success)
    (for _array_element (`KismetStringLibrary.ParseIntoArray` _unlockedscenariosonsuccess ",")
      (bind _returnvalue (`KismetStringLibrary.Conv_StringToName` _array_element))
      (bind _returnvalue_2 (`DataTableFunctionLibrary.DoesDataTableRowExist` "/Game/_Data/Scenarios/DT_Test.DT_Test" _returnvalue))
      (if _returnvalue_2
        (`KismetArrayLibrary.Array_Add` (`self.SceneQueue`) _returnvalue)
        (set `self.State` "NewEnumerator0" :!label _label)
        (else
          (`KismetSystemLibrary.PrintString` (`KismetStringLibrary.Concat_StrStr` "Data Table contains no row named: " _array_element) true true (struct :`R` 1.0 :`A` 1.0)))))
    (else
      (`KismetSystemLibrary.PrintString` _failuredialogue true true (struct :`R` 0.226087 :`B` 0.001361 :`A` 1.0))
      ; Add Unlocked Scenarios to Scene Queue (Fail)
      (for _array_element_2 (`KismetStringLibrary.ParseIntoArray` _unlockedscenariosonfailure ",")
        (bind _returnvalue_3 (`KismetStringLibrary.Conv_StringToName` _array_element_2))
        (bind _returnvalue_4 (`DataTableFunctionLibrary.DoesDataTableRowExist` "/Game/_Data/Scenarios/DT_Test.DT_Test" _returnvalue_3))
        (if _returnvalue_4
          (`KismetArrayLibrary.Array_Add` (`self.SceneQueue`) _returnvalue_3)
          (goto _label)
          (else
            (`KismetSystemLibrary.PrintString` (`KismetStringLibrary.Concat_StrStr` "Data Table contains no row named: " _array_element_2) true true (struct :`R` 1.0 :`A` 1.0))))))))

(fn `UserConstructionScript`)