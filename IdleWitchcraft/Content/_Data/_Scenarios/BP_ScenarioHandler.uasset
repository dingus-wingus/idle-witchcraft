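; Runs the game's customer scenarios: dialogue, potion hand-over, stat check and outcome.
; A state machine on the Continue button pops DT_Scenarios rows from a queue and types out dialogue via a delay loop.
; The potion's stats, weighted by scene multipliers, set the odds, with guaranteed success at the required points.
; Outcomes queue unlocked scenes, but failures first retry the check against any remaining DT_AltConditions rows.
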(event `SetDialogue`
  (params (Text :type String))
  ; Type Out Dialogue
  (set `self.TypingDialogue` true)
  (set `self.DialogueLength` 0)
  (set `self.CurrentDialogue` Text)
  (`KismetSystemLibrary.Delay` 0.0125 :!label _label)
  (`|ExecutionSequence`
    (:`then_0`
      (`/Engine/EditorBlueprintResources/StandardMacros.IncrementInt` (`self.DialogueLength`)
        (:`  `
          (`TextBlock.SetText` (`self.Dialogue`) (`KismetTextLibrary.Conv_StringToText` (`KismetStringLibrary.GetSubstring` (`self.CurrentDialogue`) 0 (+ (`self.DialogueLength`) 1)))))))
    (:`then_1`
      (if (>= (`self.DialogueLength`) (`KismetStringLibrary.Len` (`self.CurrentDialogue`)))
        (set `self.TypingDialogue` false)
        (else
          (goto _label))))))

(event `OnPotionReceived`
  (params (Potion :type "/Game/_Blueprints/_Structures/Struct_ItemStats Structure"))
  (bind _name (break `/Game/_Blueprints/_Structures/Struct_ItemStats` Potion))
  (set `self.Potion` Potion)
  (`KismetSystemLibrary.PrintString` (`KismetStringLibrary.Concat_StrStr` "Potion of " _name))
  ;[0 0.004851 0.15 0.5] Add discovered potion to array
  (`KismetArrayLibrary.Array_Add` (`self.discoveredPotions`) _name))

(event `self.ReceiveBeginPlay`
  (set `PlayerController.bShowMouseCursor` true (`GameplayStatics.GetPlayerController` 0))
  (`KismetSystemLibrary.DelayUntilNextTick`)
  (bind _asbp_player_controller (`/Game/_Blueprints/_MacroLibrary/BML_GetPlayerControllerACTOR.GetBPPlayerController` 10.0)
    (:`Success`
      (bind _bp_hud_core (`/Game/_Blueprints/BP_PlayerController.bP HUD Core` _asbp_player_controller))
      (set `self.B P HUD Core` _bp_hud_core)
      (bind _output_get (set `self.Scenario Widget` (`/Game/_Blueprints/BP_HUD_Core.WB Scenario` _bp_hud_core)))
      (`UserWidget.AddToViewport` _output_get 0)
      (set `self.Dialogue` (`/Game/_Data/_Scenarios/WB_Scenario.Dialogue` _output_get))
      (add `Button.OnReleased` (`/Game/_Data/_Scenarios/WB_Scenario.ContinueButton` _output_get) (`|CreateDelegate` :!event `OnContinueBtnPress`))
      (`self.PopNextScenario`))))

(event `OnContinueBtnPress`
  (bind _pointsscored (`self.PointsScored`))
  (bind (_scenarioname _charactername _introdialogue _actiondialogue _successdialogue _failuredialogue _altconditions _unlockedsuccess _unlockedfail _pointsrequired) (break `/Game/_Data/_Scenarios/F_Scenarios` (`self.CurrentScene`)))
  (bind _potionslot (`/Game/_Data/_Scenarios/WB_Scenario.PotionSlot` (`self.Scenario Widget`)))
  (if (not (`self.TypingDialogue`))
    (switch `/Game/_Data/_Scenarios/E_ScenarioState` (`self.State`)
      (:`NewEnumerator0`
        (`/Game/_Blueprints/BP_HUD_Core.ToggleScenario` (`self.B P HUD Core`)))
      (:`NewEnumerator1`
        (`self.BeginScenario`))
      (:`NewEnumerator3`
        (`|MultiGate` false true
          (:`Out 0`
            ; Accept Potion
            (`self.OpenPotionDropSlot`))
          (:`Out 1`
            (`/Game/_Blueprints/BP_HUD_Core.ClosePotionsInventory` (`self.B P HUD Core`))
            (`Image.SetBrush` _potionslot (make `SlateBrush` (struct :`SpecifiedColor` (struct :`R` 1.0 :`G` 1.0 :`B` 1.0 :`A` 1.0) :`ColorUseRule` "UseColor_Specified") "Image" "NoTile" "NoMirror" (struct :`X` 32.0 :`Y` 32.0) (struct) "/Game/_Textures/_Sprites/PotionPrompt.PotionPrompt"))
            (`Widget.SetVisibility` _potionslot "Hidden")
            (`self.SwitchStateStatCheck`))))
      (:`NewEnumerator4`
        (`|MultiGate` false true :!label _label_2
          (:`Out 0`
            ; Do Success Roll
            (if (>= _pointsscored _pointsrequired)
              (set `self.ScenarioSucceeded` true :!label _label_3)
              (elif (<= (`KismetMathLibrary.RandomIntegerInRange` 1 _pointsrequired) _pointsscored)
                (goto _label_3)
                (else
                  (set `self.ScenarioSucceeded` false))))
            (`self.ResolveScenario`))
          (:`Out 1`
            (`self.PopNextScenario`)
            (`/Game/_Blueprints/BP_HUD_Core.ToggleScenario` (`self.B P HUD Core`))))))
    (else
      (set `self.DialogueLength` (`KismetStringLibrary.Len` (`self.CurrentDialogue`))))))

(event `ResetStatCheck`
  (goto _label_2 :!via `Reset`))

(fn `AddScenarios`
  (params (Array :type "Array of Name"))
  ; Add Unlocked Scenarios to Scene Queue
  (for _array_element Array
    (bind _returnvalue (`DataTableFunctionLibrary.DoesDataTableRowExist` "/Game/_Data/_Scenarios/DT_Scenarios.DT_Scenarios" _array_element))
    (if _returnvalue
      (`KismetArrayLibrary.Array_Add` (`self.SceneQueue`) _array_element)
      (else
        (`KismetSystemLibrary.PrintString` (`KismetStringLibrary.Concat_StrStr` "Data Table contains no row named: " (`KismetStringLibrary.Conv_NameToString` _array_element)) true true (struct :`R` 1.0 :`A` 1.0))))))

(fn `BeginScenario`
  (bind (_currentscene_scenarioname _currentscene_charactername _currentscene_introdialogue) (break `/Game/_Data/_Scenarios/F_Scenarios` (`self.CurrentScene`)))
  (`self.SetDialogue` (`KismetStringLibrary.Concat_StrStr` _currentscene_charactername ": " _currentscene_introdialogue))
  (set `PlayerController.bShowMouseCursor` true (`PlayerState.GetPlayerController` (`GameplayStatics.GetPlayerState` 0)))
  (set `self.State` "NewEnumerator3"))

(fn `CalculateScore`
  (params (`Stat Multiplier` :type "/Game/_Data/_Scenarios/F_StatMultiplier Structure (by ref)"))
  (bind (_power _endurance _dexterity _intelligence _perception _charm) (break `/Game/_Data/_Scenarios/F_StatMultiplier` `Stat Multiplier`))
  (bind (_potion_name _potion_icon _potion_amount _potion_potioninfo) (break `/Game/_Blueprints/_Structures/Struct_ItemStats` (`self.Potion`)))
  (bind (_requiredingredients _ispotion _power_2 _endurance_2 _dexterity_2 _intelligence_2 _perception_2 _charm_2) (break `/Game/_Blueprints/_Structures/Struct_PotionStats` _potion_potioninfo))
  (set `self.PointsScored` (+ (* _power _power_2) (* _endurance _endurance_2) (* _dexterity _dexterity_2) (* _intelligence _intelligence_2) (* _perception _perception_2) (* _charm _charm_2))))

(fn `DisplayStatCheck`
  (bind _potion (`self.Potion`))
  (bind (_scenarioname _charactername _introdialogue _actiondialogue _successdialogue _failuredialogue _altconditions _unlockedsuccess _unlockedfail _pointsrequired _statmultiplier) (break `/Game/_Data/_Scenarios/F_Scenarios` (`self.CurrentScene`)))
  (bind (_power _endurance _dexterity _intelligence _perception _charm) (break `/Game/_Data/_Scenarios/F_StatMultiplier` _statmultiplier))
  ; Display Score, Stats Applied, and Odds of Success
  (`self.CalculateScore` (`.StatMultiplier_130_14EB8D934C6DB420AB20B5B6A43C3D64` (break `/Game/_Data/_Scenarios/F_Scenarios` (`self.CurrentScene`))))
  (`self.SetDialogue` (`KismetStringLibrary.Concat_StrStr` (`KismetStringLibrary.Concat_StrStr` "Stat Multiplier: " (`KismetStringLibrary.Conv_IntToString` _power) "/" (`KismetStringLibrary.Conv_IntToString` _endurance) "/" (`KismetStringLibrary.Conv_IntToString` _dexterity) "/" (`KismetStringLibrary.Conv_IntToString` _intelligence) "/" (`KismetStringLibrary.Conv_IntToString` _perception) "/" (`KismetStringLibrary.Conv_IntToString` _charm)) (`KismetStringLibrary.Concat_StrStr` " \nPotion Stats: " (`KismetStringLibrary.Conv_IntToString` (`.Power_13_DCC913344AE9DF170F8F2787DCA7FEDE` (break `/Game/_Blueprints/_Structures/Struct_PotionStats` (`.PotionInfo_20_6429C20B4872AF3261BEF0AA635272BA` (break `/Game/_Blueprints/_Structures/Struct_ItemStats` _potion))))) "/" (`KismetStringLibrary.Conv_IntToString` (`.Endurance_20_1941F52447BC8AF145FD1CA69602531F` (break `/Game/_Blueprints/_Structures/Struct_PotionStats` (`.PotionInfo_20_6429C20B4872AF3261BEF0AA635272BA` (break `/Game/_Blueprints/_Structures/Struct_ItemStats` _potion))))) "/" (`KismetStringLibrary.Conv_IntToString` (`.Dexterity_21_6878A77146DE430009EC49824ED3FFEA` (break `/Game/_Blueprints/_Structures/Struct_PotionStats` (`.PotionInfo_20_6429C20B4872AF3261BEF0AA635272BA` (break `/Game/_Blueprints/_Structures/Struct_ItemStats` _potion))))) "/" (`KismetStringLibrary.Conv_IntToString` (`.Intelligence_23_91CA58DC44ACE411F9C7859A54006EB7` (break `/Game/_Blueprints/_Structures/Struct_PotionStats` (`.PotionInfo_20_6429C20B4872AF3261BEF0AA635272BA` (break `/Game/_Blueprints/_Structures/Struct_ItemStats` _potion))))) "/" (`KismetStringLibrary.Conv_IntToString` (`.Perception_24_5E6C42034161FCD6B4EC67AD8F2D6ABA` (break `/Game/_Blueprints/_Structures/Struct_PotionStats` (`.PotionInfo_20_6429C20B4872AF3261BEF0AA635272BA` (break `/Game/_Blueprints/_Structures/Struct_ItemStats` _potion))))) "/" (`KismetStringLibrary.Conv_IntToString` (`.Charm_25_77C06F4F4B57E932D2C74B9F65E62658` (break `/Game/_Blueprints/_Structures/Struct_PotionStats` (`.PotionInfo_20_6429C20B4872AF3261BEF0AA635272BA` (break `/Game/_Blueprints/_Structures/Struct_ItemStats` _potion)))))) (`KismetStringLibrary.Concat_StrStr` " \nOdds of Success: " (`KismetStringLibrary.Conv_IntToString` (`self.PointsScored`)) "/" (`KismetStringLibrary.Conv_IntToString` _pointsrequired)))))

(fn `OpenPotionDropSlot`
  (`Widget.SetVisibility` (`/Game/_Data/_Scenarios/WB_Scenario.PotionSlot` (`self.Scenario Widget`)) "Visible")
  (`/Game/_Blueprints/BP_HUD_Core.OpenPotionsInventory` (`self.B P HUD Core`))
  (set `self.Potion` (make `/Game/_Blueprints/_Structures/Struct_ItemStats` "NONE" null 0 (make `/Game/_Blueprints/_Structures/Struct_PotionStats` _))))

(fn `PopNextScenario`
  (bind _currentscenename (`self.CurrentSceneName`))
  (bind _scenequeue (`self.SceneQueue`))
  (if (`KismetArrayLibrary.Array_IsNotEmpty` _scenequeue)
    (set `self.CurrentSceneName` (`|GetArrayItem` _scenequeue))
    (`KismetArrayLibrary.Array_Remove` (`self.SceneQueue`))
    (`self.SetDialogue` "A customer is here! Press CONTINUE to speak with them")
    (set `self.State` "NewEnumerator1")
    (bind _returnvalue (`|GetDataTableRow` "/Game/_Data/_Scenarios/DT_Scenarios.DT_Scenarios" _currentscenename)
      (:`then`
        (set `self.CurrentScene` _returnvalue))
      (:`RowNotFound`
        (`KismetSystemLibrary.PrintString` (`KismetStringLibrary.Concat_StrStr` "ERROR: No Row in DT_Scenarios Named " (`KismetStringLibrary.Conv_NameToString` _currentscenename)) true true (struct :`R` 1.0 :`A` 1.0))))
    (else
      (`self.SetDialogue` "No Scenes Remaining! Thank you for playing!")
      (set `self.State` "NewEnumerator0"))))

(fn `ResolveScenario`
  (bind (_scenarioname _charactername _introdialogue _actiondialogue _successdialogue _failuredialogue _altconditions) (break `/Game/_Data/_Scenarios/F_Scenarios` (`self.CurrentScene`)))
  (bind (_scenarioname_2 _charactername_2 _introdialogue_2 _actiondialogue_2 _successdialogue_2 _failuredialogue_2 _altconditions_2 _unlockedsuccess _unlockedfail) (break `/Game/_Data/_Scenarios/F_Scenarios` (`self.CurrentScene`)))
  (bind _output (`|GetArrayItem` _altconditions))
  (if (or (`self.ScenarioSucceeded`) (`KismetArrayLibrary.Array_IsEmpty` _altconditions))
    ; Add Unlocked Scenes
    (`self.SetDialogue` (`KismetMathLibrary.SelectString` _successdialogue_2 _failuredialogue_2 (`self.ScenarioSucceeded`)))
    (`self.AddScenarios` (select `bool` (`self.ScenarioSucceeded`) :`false` _unlockedfail :`true` _unlockedsuccess))
    (else
      ; Load Next Alt Condition
      (bind _returnvalue (`|GetDataTableRow` "/Game/_Data/_Scenarios/DT_AltConditions.DT_AltConditions" _output)
        (:`then`
          (`KismetArrayLibrary.Array_Remove` (`.AltConditions_117_495F7B0F41C817ADA10116924C26E97D` (break `/Game/_Data/_Scenarios/F_Scenarios` (`self.CurrentScene`))))
          (bind (_pointsrequired _statmultiplier _successdialogue_3 _unlocksuccess) (break `/Game/_Data/_Scenarios/F_AltConditions` _returnvalue))
          (setmembers `/Game/_Data/_Scenarios/F_Scenarios` :`StructRef` (`self.CurrentScene`) :`Success Dialogue` _successdialogue_3 :`Unlocked Success` _unlocksuccess :`Points Required` _pointsrequired :`Stat Multiplier` _statmultiplier)
          (`self.SwitchStateStatCheck`))
        (:`RowNotFound`
          (`KismetSystemLibrary.PrintString` (`KismetStringLibrary.Concat_StrStr` "ERROR: No Row in DT_AltConditions Named " (`KismetStringLibrary.Conv_NameToString` _output)) true true (struct :`R` 1.0 :`A` 1.0)))))))

(fn `SwitchStateStatCheck`
  (set `self.State` "NewEnumerator4")
  (`self.DisplayStatCheck`)
  (`self.ResetStatCheck`))

(fn `UserConstructionScript`)